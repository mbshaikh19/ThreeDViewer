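; Viewer pawn that moves on a FloatingPawnMovement component and looks around through yaw and pitch axis inputs.
; Forward input moves along the controller's forward vector, while side input uses the right vector of a zero rotation, a fixed world axis rather than the view's.
; Both move events feed shared speed logic that increments MaxSpeed when its squared axis value is non-zero and otherwise resets it to a base value.
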(event `InputAxis|ForwardMove`
  (params (AxisValue :type "Float (single-precision)"))
  (bind _floatingpawnmovement (`self.FloatingPawnMovement`))
  (`self.AddMovementInput` (`self.GetActorForwardVector` (`self.GetController`)) AxisValue true)
  (bind _returnvalue (+ (`KismetMathLibrary.Square` AxisValue) (`KismetMathLibrary.Square` (stale `InputAxis|SideMove` AxisValue))))
  (if (!= _returnvalue 0.0) :!label _label
    (set `FloatingPawnMovement.MaxSpeed` (+ (`MovementComponent.GetMaxSpeed` _floatingpawnmovement) (* _returnvalue 0.5)) _floatingpawnmovement)
    (else
      (set `FloatingPawnMovement.MaxSpeed` 100.0 _floatingpawnmovement))))

(event `InputAxis|SideMove`
  (params (AxisValue :type "Float (single-precision)"))
  (`PawnMovementComponent.AddInputVector` (`self.FloatingPawnMovement`) (* (`KismetMathLibrary.GetRightVector` (struct)) AxisValue) true)
  (goto _label))

(event `InputAxis|LookAround`
  (params (AxisValue :type "Float (single-precision)"))
  (`self.AddControllerYawInput` AxisValue))

(event `InputAxis|LookUp`
  (params (AxisValue :type "Float (single-precision)"))
  (`self.AddControllerPitchInput` AxisValue))

(fn `UserConstructionScript`)