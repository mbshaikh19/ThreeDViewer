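; Runtime model importer for a viewer: the Viewer_PC import delegate opens a file dialog and loads the chosen files through Assimp.
; Each material becomes a dynamic instance of Default_mat, using embedded or on-disk textures, with a constant base color fallback.
; ProcessNodes recursively spawns collision-free StaticMeshActors and assigns those materials by index.
; It then fires the controller's callback and repositions the player using the largest scaled mesh bounds minimum.
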(event `self.ReceiveBeginPlay`
  (bind _returnvalue (`GameplayStatics.GetPlayerController` 0))
  (`self.SetOwner` _returnvalue)
  (bind _asviewer_pc (cast `/Game/Viewer_PC` _returnvalue))
  (set `self.ViewerPC` _asviewer_pc)
  (add `/Game/Viewer_PC.ImportAssetInitiated_delegate` _asviewer_pc (delegate `ImportAsset_delegate_Event_0`)))

(event `ImportAsset_delegate_Event_0`
  (bind _materials (`self.Materials`))
  (bind _output (`|GetArrayItem` _materials (`KismetArrayLibrary.Array_LastIndex` _materials)))
  (bind (_outfilenames _success) (`AssimpFunctionLibrary.OpenFileDialogue` "Import" (`BlueprintPathsLibrary.LaunchDir`)))
  (if _success
    (bind _scenes (`AssimpFunctionLibrary.ImportScenes` _outfilenames (`GameplayStatics.GetGameMode`) (`KismetMathLibrary.Or_IntInt` (`AssimpFunctionLibrary.ProcessPreset_TargetRealtime_MaxQuality`) (`AssimpFunctionLibrary.Process_ConvertToLeftHanded`) (`AssimpFunctionLibrary.PostProcess_FixInfacingNormals`))))
    (for _array_element _scenes
      (`|ExecutionSequence`
        (:`then_0`
          (for _array_element_2 (`AIScene.GetAllMaterials` _array_element)
            (bind _returnvalue (`KismetMaterialLibrary.CreateDynamicMaterialInstance` "/Game/Default_mat.Default_mat" "None" "Transient"))
            (`KismetArrayLibrary.Array_Add` (`self.Materials`) _returnvalue)
            (`|ExecutionSequence`
              (:`then_0`
                (bind _found (`self.FindAndAssingTextures` _array_element_2 _returnvalue "AiTextureType_DIFFUSE" "BaseColor" _array_element))
                (if (not _found)
                  (`MaterialInstanceDynamic.SetScalarParameterValue` _output "UseBaseColorConstant" 1.0)
                  (`MaterialInstanceDynamic.SetVectorParameterValue` _output "BaseColorConstant" (`AIMaterial.GetMaterialBaseColor` _array_element_2))))
              (:`then_1`
                (`self.FindAndAssingTextures` _array_element_2 _returnvalue "AiTextureType_NORMALS" "Normal" _array_element))
              (:`then_2`
                (`self.FindAndAssingTextures` _array_element_2 _returnvalue "AiTextureType_METALNESS" "Metallic" _array_element))
              (:`then_3`
                (`self.FindAndAssingTextures` _array_element_2 _returnvalue "AiTextureType_SHININESS" "Roughness" _array_element))
              (:`then_4`
                (`self.FindAndAssingTextures` _array_element_2 _returnvalue "AiTextureType_EMISSIVE" "Emissive" _array_element))
              (:`then_5`
                (`MaterialInstanceDynamic.SetScalarParameterValue` _returnvalue "Opacity" 1.0)))))
        (:`then_1`
          (`self.ProcessNodes` (`AIScene.GetRootNode` _array_element)))))
    (`/Game/Viewer_PC.ImportAssetCallback_delegate` (`self.ViewerPC`))
    (`self.PositionPlayer`)))

(event `PositionPlayer`
  (bind _boundvector (`self.BoundVector`))
  (`self.K2_SetActorLocation` (`GameplayStatics.GetPlayerPawn` 0) _boundvector true false)
  (`Controller.SetControlRotation` (`GameplayStatics.GetPlayerController` 0) (`KismetMathLibrary.FindLookAtRotation` (`KismetMathLibrary.MakeVector` 0.0) _boundvector)))

(fn `FindAndAssingTextures`
  (params (AssimpMaterial :type "AIMaterial Object Reference") (DynamicMaterialUnreal :type "MaterialInstanceDynamic Object Reference") (TextureType :type "EAiTextureType Enum" :default "AiTextureType_NONE") (DynamicMaterialParamName :type Name) (AssimpScene :type "AIScene Object Reference"))
  (returns (Found :type Boolean))
  (bind (_uvscale _path _returnvalue) (`AIMaterial.GetMaterialTexture` AssimpMaterial TextureType 0 "AiTextureMapping_UV"))
  (bind _returnvalue_2 (`AIScene.GetEmbeddedTexture` AssimpScene _path (`|EnumEquality` TextureType "AiTextureType_NORMALS")))
  (switch `EAssimpReturn` _returnvalue
    (:`ReturnSuccess`
      (`/Engine/EditorBlueprintResources/StandardMacros.IsValid` _returnvalue_2
        (:`Is Valid`
          (`MaterialInstanceDynamic.SetTextureParameterValue` DynamicMaterialUnreal DynamicMaterialParamName _returnvalue_2)
          (return true))
        (:`Is Not Valid`
          (bind _returnvalue_3 (`KismetRenderingLibrary.ImportFileAsTexture2D` (`KismetMathLibrary.SelectString` (`BlueprintPathsLibrary.ConvertRelativePathToFull` (`BlueprintPathsLibrary.Split` (`AIScene.FullFilePath` AssimpScene)) _path) _path (`BlueprintPathsLibrary.IsRelative` _path))))
          (if (`|EnumEquality` TextureType "AiTextureType_NORMALS")
            (`AssimpFunctionLibrary.ApplyNormalMapSettingsToTexture` _returnvalue_3))
          (`MaterialInstanceDynamic.SetTextureParameterValue` DynamicMaterialUnreal DynamicMaterialParamName _returnvalue_3)
          (return true))))
    (:`ReturnFail`
      _)
    (:`ReturnOutOfMemory`
      _))
  (return false))

(fn `GetBoundLength`
  (params (self2 :type "StaticMeshComponent Object Reference"))
  (bind _returnvalue (* (`StaticMeshComponent.GetLocalBounds` self2) 0.1))
  (bind _returnvalue_2 (`KismetMathLibrary.VSize` _returnvalue))
  (if (> _returnvalue_2 (`self.BoundLength`))
    (set `self.BoundVector` _returnvalue)
    (set `self.BoundLength` _returnvalue_2)))

(fn `ProcessNodes`
  (params (In :type "AINode Object Reference"))
  (bind _materials (`self.Materials`))
  (`|ExecutionSequence`
    (:`then_0`
      (for _array_element (`AINode.GetNodeMeshes` In)
        (bind _returnvalue (`AIMesh.GetStaticMesh` _array_element))
        (bind _returnvalue_2 (`|SpawnActorFromClass` "/Script/Engine.StaticMeshActor" (`KismetMathLibrary.ComposeTransforms` (`AINode.GetRootTransform` In) (`KismetMathLibrary.MakeTransform` (100.0 100.0 100.0))) "Undefined" "OverrideRootScale" null null))
        (bind _staticmeshcomponent (`StaticMeshActor.StaticMeshComponent` _returnvalue_2))
        (`SceneComponent.SetMobility` _staticmeshcomponent "Movable")
        (`StaticMeshComponent.SetStaticMesh` _staticmeshcomponent _returnvalue)
        (`PrimitiveComponent.SetCollisionEnabled` _staticmeshcomponent "NoCollision")
        (`self.GetBoundLength` _staticmeshcomponent)
        (bind _returnvalue_3 (`AIMesh.GetMaterialIndex` _array_element))
        (if (`KismetArrayLibrary.Array_IsValidIndex` _materials _returnvalue_3)
          (`PrimitiveComponent.SetMaterial` _staticmeshcomponent 0 (`|GetArrayItem` _materials _returnvalue_3)))))
    (:`then_1`
      (for _array_element_2 (`AINode.GetChildNodes` In)
        (`self.ProcessNodes` _array_element_2)))))

(fn `UserConstructionScript`)